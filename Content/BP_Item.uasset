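; BP_Item is an item with a name, damage and elemental type that prints a greeting and a test damage result against Air on BeginPlay.
; A custom Constructor function, called from BeginPlay, picks a random name if it is still the default.
; GetDamage doubles damage against the opposite element, found by offsetting the victim's enum index by two with modulo wraparound.
; An older switch-based opposite check remains unconnected.
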(event EventBeginPlay
  (CallFunction|Constructor)
  (Development|PrintString (Utilities|String|Append "Hello! My name is " (Variables|Default|GetName)))
  (bind _damage (CallFunction|GetDamage "NewEnumerator3"))
  (Development|PrintString (Utilities|String|Append "our elem type is " (Utilities|String|EnumtoString (Variables|Default|GetElementalType)) ", victim is air, damage = " (Utilities|String|ToString(Integer) _damage)) true true "(R=1.000000,G=0.000000,B=0.141482,A=1.000000)" 5.0))

(fn ConstructionScript)

(fn Constructor
  (bind _returnvalue (Utilities|String|MakeLiteralString "Jalen"))
  (bind _returnvalue_2 (Utilities|String|MakeLiteralString "Brian"))
  (bind _returnvalue_3 (Utilities|String|MakeLiteralString "Gabe"))
  (bind _returnvalue_4 (Utilities|String|MakeLiteralString "Robert"))
  (bind _array (Utilities|Array|MakeArray _returnvalue_2 _returnvalue_3 _returnvalue_4 _returnvalue))
  (if (Utilities|Enum|Equal(Enum) (Variables|Default|GetName) "Item") ; randomize if name is not yet set.
    (Utilities|Array|Shuffle _array)
    (Variables|Default|SetName (Utilities|Array|Get(acopy) _array (Math|Random|RandomIntegerinRange 0 (- (Utilities|Array|Length _array) 1))))))

(fn GetDamage
  (params (VictimElemType :type ElementalType%20Enum :default "NewEnumerator1"))
  (LocalVariables|SetReturned%20Damage (Variables|Default|GetDamage)) ; set returned damage to this item's damage.
  (if (== (Class|KismetMathLibrary|PercentByteByte (+ VictimElemType 2) 4) (Math|Conversions|ToInteger(Byte) (Variables|Default|GetElementalType)))
    (LocalVariables|SetReturned%20Damage (* (Variables|Default|GetDamage) 2)))
  (return (LocalVariables|GetReturned%20Damage)))